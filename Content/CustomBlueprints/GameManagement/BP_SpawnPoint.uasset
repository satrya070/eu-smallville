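; Spinning checkpoint pickup that sets the game's respawn point when its Cube is overlapped.
; Tick adds a fixed yaw step every frame, so spin speed depends on frame rate.
; Any overlap, with no actor filter, writes its location and scale with zeroed rotation to RespawnPoint on BP_ProjectSmallVilleGameMode, prints a confirmation and destroys the actor, making it single-use.
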(event `self.ReceiveTick`
  (params (DeltaSeconds :type "Float (single-precision)"))
  (bind (_returnvalue_roll _returnvalue_pitch _returnvalue_yaw) (`KismetMathLibrary.BreakRotator` (`self.K2_GetActorRotation`)))
  (`self.K2_SetActorRotation` (`KismetMathLibrary.MakeRotator` _returnvalue_roll _returnvalue_pitch (+ _returnvalue_yaw 5.0))))

(event `self.Cube.OnComponentBeginOverlap`
  (params (OverlappedComponent :type "PrimitiveComponent Object Reference") (OtherActor :type "Actor Object Reference") (OtherComp :type "PrimitiveComponent Object Reference") (OtherBodyIndex :type Integer) (bFromSweep :type Boolean) (SweepResult :type "HitResult Structure (by ref)"))
  (bind (_returnvalue_location _returnvalue_rotation _returnvalue_scale) (`KismetMathLibrary.BreakTransform` (`self.GetTransform`)))
  (bind _asbp_project_small_ville_game_mode (cast `/Game/BP_ProjectSmallVilleGameMode` (`GameplayStatics.GetGameMode`)))
  (set `/Game/BP_ProjectSmallVilleGameMode.RespawnPoint` (`KismetMathLibrary.MakeTransform` _returnvalue_location (`KismetMathLibrary.MakeRotator` 0.0) _returnvalue_scale) _asbp_project_small_ville_game_mode)
  (`KismetSystemLibrary.PrintString` "SpawnPoint was set!")
  (`self.K2_DestroyActor`))

(fn `UserConstructionScript`)